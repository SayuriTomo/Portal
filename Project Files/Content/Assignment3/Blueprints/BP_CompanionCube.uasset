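; BP_CompanionCube is a companion cube actor that changes color when something overlaps its Box component.
; The Construction Script creates a dynamic material instance on BaseMesh's first material slot and stores it.
; The Box overlap events set that material's CompanionCubeBase color parameter, switching it on begin overlap and setting a second fixed color on end overlap.
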(event `self.Box.OnComponentBeginOverlap`
  (params (OverlappedComponent :type "PrimitiveComponent Object Reference") (OtherActor :type "Actor Object Reference") (OtherComp :type "PrimitiveComponent Object Reference") (OtherBodyIndex :type Integer) (bFromSweep :type Boolean) (SweepResult :type "HitResult Structure (by ref)"))
  (`MaterialInstanceDynamic.SetVectorParameterValue` (`self.NewVar_0`) "CompanionCubeBase" (`KismetMathLibrary.MakeColor` 1.0 0.0 0.040652)))

(event `self.Box.OnComponentEndOverlap`
  (params (OverlappedComponent :type "PrimitiveComponent Object Reference") (OtherActor :type "Actor Object Reference") (OtherComp :type "PrimitiveComponent Object Reference") (OtherBodyIndex :type Integer))
  (`MaterialInstanceDynamic.SetVectorParameterValue` (`self.NewVar_0`) "CompanionCubeBase" (`KismetMathLibrary.MakeColor` 0.0 0.0 0.0)))

(fn `UserConstructionScript`
  (bind _returnvalue (`PrimitiveComponent.CreateDynamicMaterialInstance` (`self.BaseMesh`) 0 null "None"))
  (set `self.NewVar_0` _returnvalue))